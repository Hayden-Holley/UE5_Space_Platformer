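; BP_Door is a platformer door that opens once three button presses have been registered.
; On BeginPlay it resets its counter and binds to the OnButtonsPressed dispatcher, which increments the count each time it fires.
; When the count equals three, the Door_Movement timeline plays and drives the Door component's relative Z location from its DoorOpening track.
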(event `self.ReceiveBeginPlay`
  (set `self.AmountOfButtonsPressed` 0.0)
  (add `self.OnButtonsPressed` (delegate `ButtonsPressed`)))

(event `ButtonsPressed`
  (bind _door (`self.Door`))
  (bind (_relativelocation_x _relativelocation_y) (`KismetMathLibrary.BreakVector` (`SceneComponent.RelativeLocation` _door)))
  (`/Engine/EditorBlueprintResources/StandardMacros.IncrementFloat` (`self.AmountOfButtonsPressed`)
    (:`  `
      (if (== 3.0 (`self.AmountOfButtonsPressed`))
        (bind (_direction _door_opening) (`Timeline|Door_Movement`)
          (:`Update`
            (`SceneComponent.K2_SetRelativeTransform` _door (`KismetMathLibrary.MakeTransform` (`KismetMathLibrary.MakeVector` _relativelocation_x _relativelocation_y _door_opening)) false false)))))))

(fn `UserConstructionScript`)