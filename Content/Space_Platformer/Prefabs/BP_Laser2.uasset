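; BP_Laser2 is a space-platformer laser actor that renders a red Niagara beam with an impact effect.
; Each tick it line-traces on the Camera channel from the actor toward an endpoint computed by multiplying, not adding, its location by up vector times Distance.
; The beam ends at the blocking hit or that endpoint.
; Impact effect and collision sphere follow the hit location, with the effect visible only on hits.
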(event `self.ReceiveBeginPlay`
  (`FXSystemComponent.SetColorParameter` (`self.NiagaraLaser`) "Colour" (struct :`R` 1.0 :`A` 1.0))
  (`FXSystemComponent.SetColorParameter` (`self.NiagaraLaserImpact`) "Colour" (struct :`R` 1.0 :`A` 1.0))
  (`SceneComponent.SetVisibility` (`self.NiagaraLaser`) true false))

(event `self.ReceiveTick`
  (params (DeltaSeconds :type "Float (single-precision)"))
  (bind _returnvalue (`self.K2_GetActorLocation`))
  (bind _returnvalue_2 (* _returnvalue (* (`self.GetActorUpVector`) (`self.Distance`))))
  (set `self.TraceEnd` _returnvalue_2)
  (bind _outhit (`KismetSystemLibrary.LineTraceSingle` _returnvalue _returnvalue_2 "TraceTypeQuery2"))
  (set `self.bHit` (`GameplayStatics.BreakHitResult` _outhit))
  (set `self.HitLocation` (`.Location` (`GameplayStatics.BreakHitResult` _outhit)))
  (`FXSystemComponent.SetVectorParameter` (`self.NiagaraLaser`) "LaserEnd" (select `bool` (`self.bHit`) :`false` (`self.TraceEnd`) :`true` (`self.HitLocation`)))
  (`SceneComponent.SetVisibility` (`self.NiagaraLaserImpact`) (`self.bHit`) false)
  (`SceneComponent.K2_SetWorldLocation` (`self.NiagaraLaserImpact`) (`self.HitLocation`) false false)
  (`SceneComponent.K2_SetWorldLocation` (`self.CollisionSphere`) (`self.HitLocation`) false false))

(fn `UserConstructionScript`)